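; ParentGun is a gun Blueprint, named as a parent class, that handles fire-rate timing.
; Every Tick it sets CanFire by checking whether the time elapsed since FireTime has reached FireInterval.
; It also prints the current time, FireTime and FireInterval on screen each frame as debug output.
; The file contains no firing logic and never updates FireTime, and its construction script is empty.
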(event `self.ReceiveTick`
  (params (DeltaSeconds :type "Float (single-precision)"))
  (bind _returnvalue (`GameplayStatics.GetTimeSeconds`))
  (bind _fireinterval (`self.FireInterval`))
  (bind _firetime (`self.FireTime`))
  ;[1 1 1] Calculates fire interval
  (`KismetSystemLibrary.PrintString` (`KismetStringLibrary.Conv_DoubleToString` _returnvalue) true true (struct :`R` 0.086431 :`G` 1.0 :`A` 1.0))
  (`KismetSystemLibrary.PrintString` (`KismetStringLibrary.Conv_DoubleToString` _firetime) true true (struct :`R` 0.086431 :`G` 1.0 :`A` 1.0))
  (`KismetSystemLibrary.PrintString` (`KismetStringLibrary.Conv_DoubleToString` _fireinterval) true true (struct :`R` 0.086431 :`G` 1.0 :`A` 1.0))
  (if (>= (- _returnvalue _firetime) _fireinterval)
    (set `self.CanFire` true)
    (else
      (set `self.CanFire` false))))

(fn `UserConstructionScript`)