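; Pistol weapon Blueprint that fires a Bullet actor while owned and its trigger is pressed.
; Tick calls the parent, checks the fire flags, spawns a scaled-up Bullet at the Cube component and passes its forward X/Y, with Y offset, to FireEvent.
; Each shot clears CanFire and records FireTime; nothing in this graph re-enables firing.
; Debug prints report blocked states and the Cube's rotation every frame.
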(event `self.ReceiveTick`
  (params (DeltaSeconds :type "Float (single-precision)"))
  (bind _cube (`self.Cube`))
  (bind (_returnvalue_x _returnvalue_y _returnvalue_z) (`KismetMathLibrary.BreakVector` (`SceneComponent.K2_GetComponentLocation` _cube)))
  (bind (_returnvalue_x_2 _returnvalue_y_2) (`KismetMathLibrary.BreakVector` (`SceneComponent.GetForwardVector` _cube)))
  (`parent.ReceiveTick` DeltaSeconds)
  (`|ExecutionSequence`
    (:`then_0`
      (if (`self.Owned`)
        ;[1 1 1] Spawn Bullet
        (if (and (`self.CanFire`) (`self.IsTriggerPressed`))
          (set `self.CanFire` false)
          (bind _returnvalue (`|SpawnActorFromClass` "/Game/EthansStuff/Bullet.Bullet_C" (`KismetMathLibrary.MakeTransform` (`KismetMathLibrary.MakeVector` (+ _returnvalue_x (* _returnvalue_x_2 0.0)) _returnvalue_y _returnvalue_z) (`SceneComponent.K2_GetComponentRotation` _cube) (10.0 10.0 10.0)) "Undefined" "OverrideRootScale" null self))
          (`/Game/EthansStuff/Bullet.FireEvent` _returnvalue 0.0 (`KismetMathLibrary.MakeVector2D` _returnvalue_x_2 (+ _returnvalue_y_2 2.0)))
          (set `self.FireTime` (`GameplayStatics.GetTimeSeconds`))
          (else
            (`KismetSystemLibrary.PrintString` "Can't fire")))
        (else
          (`KismetSystemLibrary.PrintString` "Not owned" true true (struct :`G` 0.66 :`B` 1.0 :`A` 1.0) 0.01))))
    (:`then_1`
      (`KismetSystemLibrary.PrintString` (`KismetStringLibrary.Conv_RotatorToString` (`SceneComponent.K2_GetComponentRotation` _cube))))))

(fn `UserConstructionScript`
  (`parent.UserConstructionScript`))