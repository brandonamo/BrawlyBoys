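; Shotgun weapon that fires a burst of fast, short-lived bullets from its Paper2D sprite when owned and triggered.
; Tick gates firing with a DoOnce that resets on trigger release, plus CanFire and ammo checks.
; Each bullet carries the player index and gets a normalized 2D direction from the sprite's forward vector plus random, rotation-based spread.
; Each burst costs one ammo, clears CanFire and records FireTime.
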(event `self.ReceiveTick`
  (params (DeltaSeconds :type "Float (single-precision)"))
  (bind _papersprite (`self.PaperSprite`))
  (bind (_returnvalue_x _returnvalue_y) (`KismetMathLibrary.BreakVector` (`SceneComponent.GetForwardVector` _papersprite)))
  (bind (_returnvalue_roll _returnvalue_pitch) (`KismetMathLibrary.BreakRotator` (`SceneComponent.K2_GetComponentRotation` _papersprite)))
  (bind (_returnvalue_x_2 _returnvalue_y_2) (`KismetMathLibrary.BreakVector2D` (+ (`KismetMathLibrary.MakeVector2D` _returnvalue_x _returnvalue_y) (`KismetMathLibrary.MakeVector2D` (`KismetMathLibrary.RandomFloatInRange` (+ _returnvalue_roll 0.2) (- _returnvalue_roll 0.2)) (`KismetMathLibrary.RandomFloatInRange` (+ _returnvalue_pitch 0.2) (- _returnvalue_pitch 0.2))))))
  (bind (_returnvalue_x_3 _returnvalue_y_3) (`KismetMathLibrary.BreakVector` (`KismetMathLibrary.Normal` (`KismetMathLibrary.MakeVector` _returnvalue_x_2 _returnvalue_y_2))))
  (`parent.ReceiveTick` DeltaSeconds)
  (`|ExecutionSequence`
    (:`then_0`
      (if (`self.Owned`)
        (if (`self.IsTriggerPressed`)
          (`/Engine/EditorBlueprintResources/StandardMacros.DoOnce` false :!label _label
            (:`Completed`
              (if (`self.CanFire`)
                (if (> (`self.Ammo limit`) 0)
                  (for _ (range 6)
                    ;[1 1 1] Spawn Bullet
                    (bind _returnvalue (`|SpawnActorFromClass` "/Game/EthansStuff/Bullet.Bullet_C" (`KismetMathLibrary.MakeTransform` (`SceneComponent.K2_GetComponentLocation` _papersprite) (`SceneComponent.K2_GetComponentRotation` _papersprite) (10.0 10.0 10.0)) "Undefined" "OverrideRootScale" null self))
                    (set `/Game/EthansStuff/Bullet.Lifespan` 0.4 _returnvalue)
                    (set `/Game/EthansStuff/Bullet.Speed` 20000.0 _returnvalue)
                    (set `/Game/EthansStuff/Bullet.Index` (`self.PlayerIndex`) _returnvalue)
                    (`/Game/EthansStuff/Bullet.FireEvent` _returnvalue (`KismetMathLibrary.MakeVector2D` _returnvalue_x_3 _returnvalue_y_3)))
                  (set `self.CanFire` false)
                  (set `self.FireTime` (`GameplayStatics.GetTimeSeconds`))
                  (`/Engine/EditorBlueprintResources/StandardMacros.DecrementInt` (`self.Ammo limit`))))))
          (else
            (goto _label :!via `Reset`)))))))

(event `self.ReceiveBeginPlay`
  (`parent.ReceiveBeginPlay`)
  (set `self.Weapon Name` "Shotgun"))

(fn `UserConstructionScript`
  (`parent.UserConstructionScript`))